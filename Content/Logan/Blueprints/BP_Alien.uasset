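; Alien AI enemy that stalks one of two players and can cross between their P1 and P2 sides through air vents.
; Looping AIMoveTo calls roam around the target player, switching to a chase when perception updates on them and back when it forgets them.
; SwitchSides swaps targets, walks to the nearest vent, teleports to the vent nearest the new target, then hides with crawl audio before wandering again.
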(event `self.ReceiveBeginPlay`
  (bind _asbp_third_person_character_synty_logan (cast `/Game/Logan/Blueprints/BP_ThirdPersonCharacterSynty_Logan` (`GameplayStatics.GetPlayerCharacter` (`KismetMathLibrary.Conv_BoolToInt` (`self.P2Side`)))))
  (set `self.TargetedPlayer` _asbp_third_person_character_synty_logan)
  (`self.Wander`))

(event `Wander`
  (set `self.Mode` "NewEnumerator0")
  (bind _randomlocation (`NavigationSystemV1.K2_GetRandomLocationInNavigableRadius` (`self.K2_GetActorLocation` (`self.TargetedPlayer`)) 1000.0 null null :!label _label))
  (`|AIMoveTo` self _randomlocation null
    (:`OnSuccess`
      (`KismetSystemLibrary.PrintString` "Success"))
    (:`OnFail`
      (`KismetSystemLibrary.PrintString` "Fail")))
  (if (`|EnumEquality` (`self.Mode`) "NewEnumerator0")
    (goto _label)))

(event `self.ReceiveTick`
  (params (DeltaSeconds :type "Float (single-precision)")))

(event `Hunt`
  (if (`self.SwitchingSides`) :!label _label_2
    (`KismetSystemLibrary.Delay` 0.1)
    (goto _label_2)
    (else
      (`|AIMoveTo` self (0.0 0.0 0.0) (`self.TargetedPlayer`) :!label _label_3
        (:`OnSuccess`
          (`KismetSystemLibrary.PrintString` "Success"))
        (:`OnFail`
          (`KismetSystemLibrary.PrintString` "Fail")))
      (if (`|EnumEquality` (`self.Mode`) "NewEnumerator1")
        (goto _label_3)))))

(event `self.AIPerception.OnTargetPerceptionUpdated`
  (params (Actor :type "Actor Object Reference") (Stimulus :type "AIStimulus Structure"))
  (if (== Actor (`self.TargetedPlayer`))
    (`self.ResetMovement`)
    (`self.Hunt`)))

(event `self.AIPerception.OnTargetPerceptionForgotten`
  (params (Actor :type "Actor Object Reference"))
  (if (== Actor (`self.TargetedPlayer`))
    (`self.ResetMovement`)
    (`self.Wander`)))

(event `SwitchSides`
  (bind _targetedplayer (`self.TargetedPlayer`))
  (bind _returnvalue (`GameplayStatics.GetPlayerCharacter` (`KismetMathLibrary.Conv_BoolToInt` (`self.P2Side`))))
  (set `self.SwitchingSides` true)
  (if (`self.P2Side`)
    (set `self.P2Side` false)
    (bind _asbp_third_person_character_synty_logan (cast `/Game/Logan/Blueprints/BP_ThirdPersonCharacterSynty_Logan` _returnvalue))
    (set `self.TargetedPlayer` _asbp_third_person_character_synty_logan)
    (bind _outactors (`GameplayStatics.GetAllActorsOfClassWithTag` "/Game/Logan/Blueprints/BP_AirVent.BP_AirVent_C" "P2"))
    (bind _nearestvent (`self.FindNearestVent` _outactors self))
    (`|AIMoveTo` self (`self.K2_GetActorLocation` _nearestvent) null 100.0 true :!label _label_4
      (:`OnSuccess`
        (bind _outactors_2 (`GameplayStatics.GetAllActorsOfClassWithTag` "/Game/Logan/Blueprints/BP_AirVent.BP_AirVent_C" "P1"))
        (bind _nearestvent_2 (`self.FindNearestVent` _outactors_2 _targetedplayer))
        (`self.K2_SetActorLocation` (`SceneComponent.K2_GetComponentLocation` (`/Game/Logan/Blueprints/BP_AirVent.AlienTeleportPoint` _nearestvent_2)) false true))
      (:`OnFail`
        (`KismetSystemLibrary.Delay` 0.1)
        (goto _label_4)))
    (else
      (set `self.P2Side` true)
      (bind _asbp_third_person_character_synty_logan_2 (cast `/Game/Logan/Blueprints/BP_ThirdPersonCharacterSynty_Logan` _returnvalue))
      (set `self.TargetedPlayer` _asbp_third_person_character_synty_logan_2)
      (bind _outactors_3 (`GameplayStatics.GetAllActorsOfClassWithTag` "/Game/Logan/Blueprints/BP_AirVent.BP_AirVent_C" "P1"))
      (bind _nearestvent_3 (`self.FindNearestVent` _outactors_3 self))
      (`|AIMoveTo` self (`self.K2_GetActorLocation` _nearestvent_3) null 100.0 :!label _label_5
        (:`OnSuccess`
          (bind _outactors_4 (`GameplayStatics.GetAllActorsOfClassWithTag` "/Game/Logan/Blueprints/BP_AirVent.BP_AirVent_C" "P2"))
          (bind _nearestvent_4 (`self.FindNearestVent` _outactors_4 _targetedplayer))
          (`self.K2_SetActorLocation` (`SceneComponent.K2_GetComponentLocation` (`/Game/Logan/Blueprints/BP_AirVent.AlienTeleportPoint` _nearestvent_4)) false true))
        (:`OnFail`
          (`KismetSystemLibrary.Delay` 0.1)
          (goto _label_5)))))
  (`CharacterMovementComponent.DisableMovement` (`self.CharacterMovement`))
  (`SceneComponent.SetVisibility` (`self.Mesh1`) false false)
  (bind _returnvalue_2 (`GameplayStatics.SpawnSoundAtLocation` "/Game/Logan/Audio/Air_Duct_Crawl_⧸_Through__Metal__Impact-eB3LrY1dJVM.Air_Duct_Crawl_⧸_Through__Metal__Impact-eB3LrY1dJVM" (`self.K2_GetActorLocation`) (struct) 1.0 1.0 0.0 null null))
  (`KismetSystemLibrary.Delay` 10.0)
  (`SceneComponent.SetVisibility` (`self.Mesh1`) true false)
  (`AudioComponent.Stop` _returnvalue_2)
  (set `self.SwitchingSides` false)
  (`self.ResetMovement`)
  (`self.Wander`))

(fn `FindNearestVent`
  (params (Vents :type "Array of /Game/Logan/Blueprints/BP_AirVent Object Reference") (TargetActor :type "Actor Object Reference"))
  (returns (NearestVent :type "/Game/Logan/Blueprints/BP_AirVent Object Reference"))
  (locals (ChosenVent :type "/Game/Logan/Blueprints/BP_AirVent Object Reference"))
  (set `local.ChosenVent` (`|GetArrayItem` Vents))
  (for _array_element Vents
    (if (< (`KismetMathLibrary.Vector_Distance` (`self.K2_GetActorLocation` _array_element) (`self.K2_GetActorLocation` (`local.TargetActor`))) (`KismetMathLibrary.Vector_Distance` (`self.K2_GetActorLocation` (`local.ChosenVent`)) (`self.K2_GetActorLocation` (`local.TargetActor`))))
      (set `local.ChosenVent` _array_element)))
  (return (`local.ChosenVent`)))

(fn `ResetMovement`
  (bind _charactermovement (`self.CharacterMovement`))
  (set `self.Mode` "NewEnumerator1")
  (`CharacterMovementComponent.DisableMovement` _charactermovement)
  (`CharacterMovementComponent.SetMovementMode` _charactermovement "MOVE_Walking" 0))

(fn `UserConstructionScript`)