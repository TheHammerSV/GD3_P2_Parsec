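; BP_SignalDoor_Final is a door that swings open when its SignalRecieved event fires.
; BeginPlay caches the door's starting relative rotation.
; The signal plays a spaceship door sound at world origin and runs a timeline that lerps yaw up to 140 degrees beyond the cached yaw, zeroing pitch and roll.
; The graph has no closing logic.
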(event `self.ReceiveBeginPlay`
  (set `self.DefaultDoorRotation` (`SceneComponent.RelativeRotation` (`self.Door`))))

(event `SignalRecieved`
  (bind (_defaultdoorrotation_roll _defaultdoorrotation_pitch _defaultdoorrotation_yaw) (`KismetMathLibrary.BreakRotator` (`self.DefaultDoorRotation`)))
  (`GameplayStatics.PlaySoundAtLocation` "/Game/Ricardo/KeyCardAndDoor/Door_Sounds/spaceship-door-opening-43604.spaceship-door-opening-43604" (0.0 0.0 0.0) (struct) 1.0 1.0 0.0 null null null null)
  (bind (_direction _open_door) (`Timeline|Timeline`)
    (:`Update`
      (`SceneComponent.K2_SetRelativeRotation` (`self.Door`) (`KismetMathLibrary.MakeRotator` 0.0 0.0 (+ (`KismetMathLibrary.Lerp` 0.0 140.0 _open_door) _defaultdoorrotation_yaw)) false false))))

(fn `UserConstructionScript`)