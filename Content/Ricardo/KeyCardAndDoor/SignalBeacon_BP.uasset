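; SignalBeacon_BP is a beacon that lets the player send a one-time signal to the level's signal doors.
; Overlap of its box by the Ricardo third-person character enables input and opens a Gate; leaving disables input and closes it.
; While inside, the Signal Door input passes through the Gate and a DoOnce, then calls SignalRecieved on every SignalDoor_BP, with debug prints.
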(event `self.ReceiveBeginPlay`)

(event `InputAction|Signal Door`
  (params (Key :type "Key Structure"))
  (:`Pressed`
    (`KismetSystemLibrary.PrintString` "Click")
    (`/Engine/EditorBlueprintResources/StandardMacros.Gate` true :!label _label
      (:`Exit`
        (`/Engine/EditorBlueprintResources/StandardMacros.DoOnce` false
          (:`Completed`
            (bind _outactors (`GameplayStatics.GetAllActorsOfClass` "/Game/Ricardo/KeyCardAndDoor/SignalDoor_BP.SignalDoor_BP_C"))
            (`/Game/Ricardo/KeyCardAndDoor/SignalDoor_BP.SignalRecieved` _outactors)
            (`KismetSystemLibrary.PrintString` "Signal")))))))

(event `self.Box.OnComponentBeginOverlap`
  (params (OverlappedComponent :type "PrimitiveComponent Object Reference") (OtherActor :type "Actor Object Reference") (OtherComp :type "PrimitiveComponent Object Reference") (OtherBodyIndex :type Integer) (bFromSweep :type Boolean) (SweepResult :type "HitResult Structure (by ref)"))
  (cast `/Game/Ricardo/BP_ThirdPersonCharacterSynty_Ric` OtherActor)
  (`self.EnableInput` (`GameplayStatics.GetPlayerController` 0))
  (goto _label :!via `Open`))

(event `self.Box.OnComponentEndOverlap`
  (params (OverlappedComponent :type "PrimitiveComponent Object Reference") (OtherActor :type "Actor Object Reference") (OtherComp :type "PrimitiveComponent Object Reference") (OtherBodyIndex :type Integer))
  (cast `/Game/Ricardo/BP_ThirdPersonCharacterSynty_Ric` OtherActor)
  (`self.DisableInput` (`GameplayStatics.GetPlayerController` 0))
  (goto _label :!via `Close`))

(fn `UserConstructionScript`)