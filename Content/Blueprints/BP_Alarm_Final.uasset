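; Interactable alarm that a player can use to make the alien switch sides.
; On Use it removes that player's interaction widget and looks up the BP_Alien_Final actor in the level.
; If the alien exists and is targeting someone other than the user, it calls SwitchSides on it and plays an alarm sound at the alarm's location.
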(event `self.Use`
  (params (Player :type "/Game/Blueprints/BP_ThirdPersonCharacterSynty_Final Object Reference"))
  (`Widget.RemoveFromParent` (`/Game/Blueprints/BP_ThirdPersonCharacterSynty_Final.InteractableWidget` Player))
  (bind _returnvalue (`GameplayStatics.GetActorOfClass` "/Game/Blueprints/BP_Alien_Final.BP_Alien_Final_C"))
  (`/Engine/EditorBlueprintResources/StandardMacros.IsValid` _returnvalue
    (:`Is Valid`
      (if (!= (`/Game/Blueprints/BP_Alien_Final.TargetedPlayer` _returnvalue) Player)
        (`/Game/Blueprints/BP_Alien_Final.SwitchSides` _returnvalue)
        (`GameplayStatics.PlaySoundAtLocation` "/Game/Logan/Audio/Alarm-Slow-A1-www_fesliyanstudios_com.Alarm-Slow-A1-www_fesliyanstudios_com" (`self.K2_GetActorLocation`) (struct) 1.0 1.0 0.0 null null null null)))))

(fn `UserConstructionScript`
  (`parent.UserConstructionScript`))