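; BP_Door2_Final is a double door that opens once the player holds KeyCard2.
; Tick sets the prompt text from the player character's key card state and clears it once the door is open.
; Use checks the card, removes the player's interact widget, then plays a sound at world origin and a Timeline that slides both panels along relative X from their BeginPlay positions.
; The door has no closing logic.
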(event `self.ReceiveBeginPlay`
  (set `self.DoorStartPos` (`SceneComponent.RelativeLocation` (`self.Door`)))
  (set `self.Door2StartPos` (`SceneComponent.RelativeLocation` (`self.Door2`))))

(event `self.ReceiveTick`
  (params (DeltaSeconds :type "Float (single-precision)"))
  (bind _asbp_third_person_character_synty_final (cast `/Game/Blueprints/BP_ThirdPersonCharacterSynty_Final` (`GameplayStatics.GetPlayerCharacter` (`self.PlayerIndex`))))
  (if (`self.Open`)
    (set `self.WidgetText` "")
    (elif (`/Game/Blueprints/BP_ThirdPersonCharacterSynty_Final.KeyCard2` _asbp_third_person_character_synty_final)
      (set `self.WidgetText` "Press E to Open Door")
      (else
        (set `self.WidgetText` "Find Key Card to Open Door")))))

(event `self.Use`
  (params (Player :type "/Game/Blueprints/BP_ThirdPersonCharacterSynty_Final Object Reference"))
  (bind _doorstartpos_x (`KismetMathLibrary.BreakVector` (`self.DoorStartPos`)))
  (bind _door2startpos_x (`KismetMathLibrary.BreakVector` (`self.Door2StartPos`)))
  (if (and (== (`/Game/Blueprints/BP_ThirdPersonCharacterSynty_Final.KeyCard2` Player) true) (== (`self.Open`) false))
    (set `self.Open` true)
    (`Widget.RemoveFromParent` (`/Game/Blueprints/BP_ThirdPersonCharacterSynty_Final.InteractableWidget` Player))
    (`/Engine/EditorBlueprintResources/StandardMacros.DoOnce` false
      (:`Completed`
        (`GameplayStatics.PlaySoundAtLocation` "/Game/Ricardo/KeyCardAndDoor/Door_Sounds/door-open-107728.door-open-107728" (0.0 0.0 0.0) (struct) 1.0 1.0 0.0 null null null null)
        (bind (_direction _door _door2) (`Timeline|Timeline`)
          (:`Update`
            (`|ExecutionSequence`
              (:`then_0`
                (`SceneComponent.K2_SetRelativeTransform` (`self.Door`) (`KismetMathLibrary.MakeTransform` (`KismetMathLibrary.MakeVector` (+ _door _doorstartpos_x))) false false))
              (:`then_1`
                (`SceneComponent.K2_SetRelativeTransform` (`self.Door2`) (`KismetMathLibrary.MakeTransform` (`KismetMathLibrary.MakeVector` (+ _door2 _door2startpos_x))) false false)))))))))

(fn `UserConstructionScript`)