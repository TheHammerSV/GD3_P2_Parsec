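; BP_FixArea_Final is an interactable ship repair point that the player fixes by spending scrap.
; Tick sets the prompt text from the fixed state and the overlapping player's scrap count.
; Use checks for scrap and an unfixed state, then deducts scrap, removes the prompt widget and plays a sound.
; It also reveals the Fixed component and destroys the point light and Broken component.
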(event `self.ReceiveTick`
  (params (DeltaSeconds :type "Float (single-precision)"))
  (bind _overlappedplayer (`self.OverlappedPlayer`))
  (if (`self.IsFixed`)
    (set `self.WidgetText` "")
    (else
      (`/Engine/EditorBlueprintResources/StandardMacros.IsValid` _overlappedplayer
        (:`Is Valid`
          (if (> (`/Game/Blueprints/BP_ThirdPersonCharacterSynty_Final.Scrap` _overlappedplayer) 0.0)
            (set `self.WidgetText` "Press E to Fix")
            (else
              (set `self.WidgetText` "Find Scrap to Fix"))))))))

(event `self.Use`
  (params (Player :type "/Game/Blueprints/BP_ThirdPersonCharacterSynty_Final Object Reference"))
  (if (and (> (`/Game/Blueprints/BP_ThirdPersonCharacterSynty_Final.Scrap` Player) 0.0) (== (`self.IsFixed`) false))
    (set `self.IsFixed` true)
    (`/Engine/EditorBlueprintResources/StandardMacros.DecrementFloat` (`/Game/Blueprints/BP_ThirdPersonCharacterSynty_Final.Scrap` Player)
      (:`  `
        (`Widget.RemoveFromParent` (`/Game/Blueprints/BP_ThirdPersonCharacterSynty_Final.InteractableWidget` Player))
        (`GameplayStatics.PlaySoundAtLocation` null (0.0 0.0 0.0) (struct) 1.0 1.0 0.0 null null null null)
        (`SceneComponent.SetVisibility` (`self.Fixed`) true false)
        (`ActorComponent.K2_DestroyComponent` (`self.PointLight`))
        (`ActorComponent.K2_DestroyComponent` (`self.Broken`))
        (`KismetSystemLibrary.PrintString` "Fixed")))))

(fn `UserConstructionScript`)