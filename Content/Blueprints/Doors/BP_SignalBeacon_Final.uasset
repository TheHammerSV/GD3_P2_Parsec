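; BP_SignalBeacon_Final is an interactable switch that opens remote doors once, showing a prompt until used.
; Box overlap by the player character toggles that player's input and a Gate.
; Use sets Open and removes the player's widget before passing through the Gate and a DoOnce to call SignalRecieved on ConnectedDoors, so Open is set even if the Gate is closed.
; Tick refreshes the prompt text from Open.
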(event `self.ReceiveBeginPlay`)

(event `self.ReceiveTick`
  (params (DeltaSeconds :type "Float (single-precision)"))
  (if (`self.Open`)
    (set `self.WidgetText` "")
    (else
      (set `self.WidgetText` "Press E To Open Remote Door"))))

(event `self.Use`
  (params (Player :type "/Game/Blueprints/BP_ThirdPersonCharacterSynty_Final Object Reference"))
  (if (not (`self.Open`))
    (set `self.Open` true)
    (`Widget.RemoveFromParent` (`/Game/Blueprints/BP_ThirdPersonCharacterSynty_Final.InteractableWidget` Player))
    (`KismetSystemLibrary.PrintString` "Click")
    (`/Engine/EditorBlueprintResources/StandardMacros.Gate` true :!label _label
      (:`Exit`
        (`/Engine/EditorBlueprintResources/StandardMacros.DoOnce` false
          (:`Completed`
            (for _array_element (`self.ConnectedDoors`)
              (`/Game/Blueprints/Doors/BP_SignalDoor_Final.SignalRecieved` _array_element))))))))

(event `self.Box.OnComponentBeginOverlap`
  (params (OverlappedComponent :type "PrimitiveComponent Object Reference") (OtherActor :type "Actor Object Reference") (OtherComp :type "PrimitiveComponent Object Reference") (OtherBodyIndex :type Integer) (bFromSweep :type Boolean) (SweepResult :type "HitResult Structure (by ref)"))
  (bind _asbp_third_person_character_synty_final (cast `/Game/Blueprints/BP_ThirdPersonCharacterSynty_Final` OtherActor))
  (`self.EnableInput` (`GameplayStatics.GetPlayerController` (`/Game/Blueprints/BP_ThirdPersonCharacterSynty_Final.Index` _asbp_third_person_character_synty_final)))
  (goto _label :!via `Open`))

(event `self.Box.OnComponentEndOverlap`
  (params (OverlappedComponent :type "PrimitiveComponent Object Reference") (OtherActor :type "Actor Object Reference") (OtherComp :type "PrimitiveComponent Object Reference") (OtherBodyIndex :type Integer))
  (bind _asbp_third_person_character_synty_final (cast `/Game/Blueprints/BP_ThirdPersonCharacterSynty_Final` OtherActor))
  (`self.DisableInput` (`GameplayStatics.GetPlayerController` (`/Game/Blueprints/BP_ThirdPersonCharacterSynty_Final.Index` _asbp_third_person_character_synty_final)))
  (goto _label :!via `Close`))

(fn `UserConstructionScript`)