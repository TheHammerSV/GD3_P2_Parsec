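; BP_Switch_Entrance_Final is an interactable key card sender that passes the player's cards to BP_Switch_Exit_Final.
; Tick sets the prompt text according to whether the player character holds any of three key cards.
; On Use, each held card's flag is cleared and its matching function is called on the exit switch.
; A shared timeline rotates the box lid and shows a point light until finished, alongside a door sound.
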(event `self.ReceiveTick`
  (params (DeltaSeconds :type "Float (single-precision)"))
  (bind _asbp_third_person_character_synty_final (cast `/Game/Blueprints/BP_ThirdPersonCharacterSynty_Final` (`GameplayStatics.GetPlayerCharacter` (`self.Side`))))
  (if (and (== (`/Game/Blueprints/BP_ThirdPersonCharacterSynty_Final.KeyCard` _asbp_third_person_character_synty_final) false) (== (`/Game/Blueprints/BP_ThirdPersonCharacterSynty_Final.KeyCard2` _asbp_third_person_character_synty_final) false) (== (`/Game/Blueprints/BP_ThirdPersonCharacterSynty_Final.KeyCard3` _asbp_third_person_character_synty_final) false))
    (set `self.WidgetText` "Collect key card to use")
    (else
      (set `self.WidgetText` "Press E To Send Key Card"))))

(event `self.Use`
  (params (Player :type "/Game/Blueprints/BP_ThirdPersonCharacterSynty_Final Object Reference"))
  (bind _returnvalue (`GameplayStatics.GetActorOfClass` "/Game/Blueprints/BP_Switch_Exit_Final.BP_Switch_Exit_Final_C"))
  (`|ExecutionSequence`
    (:`then_0`
      (if (`/Game/Blueprints/BP_ThirdPersonCharacterSynty_Final.KeyCard` Player)
        (set `/Game/Blueprints/BP_ThirdPersonCharacterSynty_Final.KeyCard` false Player)
        (`/Game/Blueprints/BP_Switch_Exit_Final.Keycard 1` _returnvalue)
        (`|ExecutionSequence` :!label _label
          (:`then_0`
            (bind (_direction _lid_shut) (`Timeline|LidShut` :!via `PlayFromStart`)
              (:`Update`
                (`SceneComponent.K2_SetRelativeRotation` (`self.BoxLid`) (`KismetMathLibrary.MakeRotator` _lid_shut) false false)
                (`SceneComponent.SetVisibility` (`self.PointLight`) true false))
              (:`Finished`
                (`SceneComponent.SetVisibility` (`self.PointLight`) false false))))
          (:`then_1`
            (`GameplayStatics.PlaySoundAtLocation` "/Game/Ricardo/Switch_BP/door-43633.door-43633" (`SceneComponent.RelativeLocation` (`self.BoxLid`)) (struct) 1.0 1.0 0.0 null null null null)))))
    (:`then_1`
      (if (`/Game/Blueprints/BP_ThirdPersonCharacterSynty_Final.KeyCard2` Player)
        (set `/Game/Blueprints/BP_ThirdPersonCharacterSynty_Final.KeyCard2` false Player)
        (`/Game/Blueprints/BP_Switch_Exit_Final.KeyCard 2` _returnvalue)
        (goto _label)))
    (:`then_2`
      (if (`/Game/Blueprints/BP_ThirdPersonCharacterSynty_Final.KeyCard3` Player)
        (set `/Game/Blueprints/BP_ThirdPersonCharacterSynty_Final.KeyCard3` false Player)
        (`/Game/Blueprints/BP_Switch_Exit_Final.KeyCard 3` _returnvalue)
        (goto _label)))))

(fn `UserConstructionScript`)