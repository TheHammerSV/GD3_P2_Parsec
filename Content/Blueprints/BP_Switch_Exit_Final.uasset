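; BP_Switch_Exit_Final is an actor that dispenses one of three exit keycards when the matching custom event is called.
; Each event plays a vent sound at the mesh's relative location, waits, then spawns its keycard class at the Sphere's world location.
; It then reveals the point light in that card's color: blue, orange or red.
; Each event also looks up the player character but leaves the result unused.
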(event `Keycard 1`
  (bind _pointlight (`self.PointLight`))
  (`GameplayStatics.PlaySoundAtLocation` "/Game/Ricardo/Switch_BP/Vent_mixdown.Vent_mixdown" (`SceneComponent.RelativeLocation` (`self.StaticMesh`)) (struct) 1.0 1.0 0.0 null null null null)
  (`KismetSystemLibrary.Delay` 6.0)
  (`|SpawnActorFromClass` "/Game/Blueprints/Doors/BP_KeyCard1_Final.BP_KeyCard1_Final_C" (`KismetMathLibrary.MakeTransform` (`SceneComponent.K2_GetComponentLocation` (`self.Sphere`))) "AdjustIfPossibleButAlwaysSpawn" "MultiplyWithRoot" null null)
  (`GameplayStatics.GetActorOfClass` "/Game/Blueprints/BP_ThirdPersonCharacterSynty_Final.BP_ThirdPersonCharacterSynty_Final_C")
  (`SceneComponent.SetVisibility` _pointlight true false)
  (`LightComponent.SetLightColor` _pointlight (struct :`G` 0.1261 :`B` 0.619792 :`A` 1.0) true))

(event `KeyCard 2`
  (bind _pointlight (`self.PointLight`))
  (`GameplayStatics.PlaySoundAtLocation` "/Game/Ricardo/Switch_BP/Vent_mixdown.Vent_mixdown" (`SceneComponent.RelativeLocation` (`self.StaticMesh`)) (struct) 1.0 1.0 0.0 null null null null)
  (`KismetSystemLibrary.Delay` 6.0)
  (`|SpawnActorFromClass` "/Game/Blueprints/Doors/BP_KeyCard2_Final.BP_KeyCard2_Final_C" (`KismetMathLibrary.MakeTransform` (`SceneComponent.K2_GetComponentLocation` (`self.Sphere`))) "AdjustIfPossibleButAlwaysSpawn" "MultiplyWithRoot" null null)
  (`GameplayStatics.GetActorOfClass` "/Game/Blueprints/BP_ThirdPersonCharacterSynty_Final.BP_ThirdPersonCharacterSynty_Final_C")
  (`SceneComponent.SetVisibility` _pointlight true false)
  (`LightComponent.SetLightColor` _pointlight (struct :`R` 0.619792 :`G` 0.350094 :`A` 1.0) true))

(event `KeyCard 3`
  (bind _pointlight (`self.PointLight`))
  (`GameplayStatics.PlaySoundAtLocation` "/Game/Ricardo/Switch_BP/Vent_mixdown.Vent_mixdown" (`SceneComponent.RelativeLocation` (`self.StaticMesh`)) (struct) 1.0 1.0 0.0 null null null null)
  (`KismetSystemLibrary.Delay` 6.0)
  (`|SpawnActorFromClass` "/Game/Blueprints/Doors/BP_KeyCard3_Final.BP_KeyCard3_Final_C" (`KismetMathLibrary.MakeTransform` (`SceneComponent.K2_GetComponentLocation` (`self.Sphere`))) "AdjustIfPossibleButAlwaysSpawn" "MultiplyWithRoot" null null)
  (`GameplayStatics.GetActorOfClass` "/Game/Blueprints/BP_ThirdPersonCharacterSynty_Final.BP_ThirdPersonCharacterSynty_Final_C")
  (`SceneComponent.SetVisibility` _pointlight true false)
  (`LightComponent.SetLightColor` _pointlight (struct :`R` 0.505208 :`B` 0.008771 :`A` 1.0) true))

(fn `UserConstructionScript`)