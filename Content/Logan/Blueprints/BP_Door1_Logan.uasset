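; BP_Door1_Logan is a key-card-locked door that the player opens through a Use event.
; Tick casts the player character to BP_ThirdPersonCharacterSynty_Logan and sets the prompt text according to whether it holds the KeyCard.
; With the card, Use passes a DoOnce, plays a sound at the world origin and runs a Timeline that moves the mesh along relative Z, with no closing logic.
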(event `self.ReceiveTick`
  (params (DeltaSeconds :type "Float (single-precision)"))
  (bind _asbp_third_person_character_synty_logan (cast `/Game/Logan/Blueprints/BP_ThirdPersonCharacterSynty_Logan` (`GameplayStatics.GetPlayerCharacter` (`self.PlayerIndex`))))
  (if (`/Game/Logan/Blueprints/BP_ThirdPersonCharacterSynty_Logan.KeyCard` _asbp_third_person_character_synty_logan)
    (set `self.WidgetText` "Press E to Open Door")
    (else
      (set `self.WidgetText` "Find Key Card to Open Door"))))

(event `self.Use`
  (params (Player :type "/Game/Logan/Blueprints/BP_ThirdPersonCharacterSynty_Logan Object Reference"))
  (if (`/Game/Logan/Blueprints/BP_ThirdPersonCharacterSynty_Logan.KeyCard` Player)
    (`/Engine/EditorBlueprintResources/StandardMacros.DoOnce` false
      (:`Completed`
        (`GameplayStatics.PlaySoundAtLocation` "/Game/Ricardo/KeyCardAndDoor/Door_Sounds/door-open-107728.door-open-107728" (0.0 0.0 0.0) (struct) 1.0 1.0 0.0 null null null null)
        (bind (_direction _door) (`Timeline|Timeline`)
          (:`Update`
            (`SceneComponent.K2_SetRelativeTransform` (`self.Mesh`) (`KismetMathLibrary.MakeTransform` (`KismetMathLibrary.MakeVector` 0.0 0.0 _door)) false false)))))))

(fn `UserConstructionScript`
  (`parent.UserConstructionScript`))