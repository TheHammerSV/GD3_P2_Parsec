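; Key-card-locked door that slides its mesh vertically when the player uses it.
; Tick reads the player character's KeyCard flag to set the prompt text, which clears once the door is open.
; Use requires the key card, removes the player's interact widget, then fires a one-time open sound at world origin and a Timeline driving the mesh's relative Z.
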(event `self.ReceiveTick`
  (params (DeltaSeconds :type "Float (single-precision)"))
  (bind _asbp_third_person_character_synty_final (cast `/Game/Blueprints/BP_ThirdPersonCharacterSynty_Final` (`GameplayStatics.GetPlayerCharacter` (`self.PlayerIndex`))))
  (if (`self.Open`)
    (set `self.WidgetText` "")
    (elif (`/Game/Blueprints/BP_ThirdPersonCharacterSynty_Final.KeyCard` _asbp_third_person_character_synty_final)
      (set `self.WidgetText` "Press E to Open Door")
      (else
        (set `self.WidgetText` "Find Key Card to Open Door")))))

(event `self.Use`
  (params (Player :type "/Game/Blueprints/BP_ThirdPersonCharacterSynty_Final Object Reference"))
  (if (and (== (`/Game/Blueprints/BP_ThirdPersonCharacterSynty_Final.KeyCard` Player) true) (== (`self.Open`) false))
    (set `self.Open` true)
    (`Widget.RemoveFromParent` (`/Game/Blueprints/BP_ThirdPersonCharacterSynty_Final.InteractableWidget` Player))
    (`/Engine/EditorBlueprintResources/StandardMacros.DoOnce` false
      (:`Completed`
        (`GameplayStatics.PlaySoundAtLocation` "/Game/Ricardo/KeyCardAndDoor/Door_Sounds/door-open-107728.door-open-107728" (0.0 0.0 0.0) (struct) 1.0 1.0 0.0 null null null null)
        (bind (_direction _door) (`Timeline|Timeline`)
          (:`Update`
            (`SceneComponent.K2_SetRelativeTransform` (`self.Mesh`) (`KismetMathLibrary.MakeTransform` (`KismetMathLibrary.MakeVector` 0.0 0.0 _door)) false false)))))))

(fn `UserConstructionScript`
  (`parent.UserConstructionScript`))