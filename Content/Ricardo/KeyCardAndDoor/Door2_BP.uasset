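; Door2_BP is a two-part sliding door that opens for a player character holding the second key card.
; When that character begins overlapping the Box, a KeyCard2 check leads through a DoOnce, so the door opens once and has no closing logic.
; It plays an opening sound at the world origin and runs a Timeline whose two tracks drive the relative X location of Door and Door2.
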(event `self.Box.OnComponentBeginOverlap`
  (params (OverlappedComponent :type "PrimitiveComponent Object Reference") (OtherActor :type "Actor Object Reference") (OtherComp :type "PrimitiveComponent Object Reference") (OtherBodyIndex :type Integer) (bFromSweep :type Boolean) (SweepResult :type "HitResult Structure (by ref)"))
  (bind _asbp_third_person_character_synty_ric (cast `/Game/Ricardo/BP_ThirdPersonCharacterSynty_Ric` OtherActor))
  (if (`/Game/Ricardo/BP_ThirdPersonCharacterSynty_Ric.KeyCard2` _asbp_third_person_character_synty_ric)
    (`/Engine/EditorBlueprintResources/StandardMacros.DoOnce` false
      (:`Completed`
        (`GameplayStatics.PlaySoundAtLocation` "/Game/Ricardo/KeyCardAndDoor/Door_Sounds/door-open-107728.door-open-107728" (0.0 0.0 0.0) (struct) 1.0 1.0 0.0 null null null null)
        (bind (_direction _door _door2) (`Timeline|Timeline`)
          (:`Update`
            (`|ExecutionSequence`
              (:`then_0`
                (`SceneComponent.K2_SetRelativeTransform` (`self.Door`) (`KismetMathLibrary.MakeTransform` (`KismetMathLibrary.MakeVector` _door)) false false))
              (:`then_1`
                (`SceneComponent.K2_SetRelativeTransform` (`self.Door2`) (`KismetMathLibrary.MakeTransform` (`KismetMathLibrary.MakeVector` _door2)) false false)))))))))

(fn `UserConstructionScript`)