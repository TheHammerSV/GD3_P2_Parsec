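; Game mode for local two-player play that sets up both characters when play begins.
; It creates a second local player and adds the Player 2 Enhanced Input mapping context to that controller.
; Each Synty third-person character gets an index of 0 or 1 and is teleported to the PlayerStart tagged P1 or P2.
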(event `self.ReceiveBeginPlay`
  (bind _returnvalue (`GameplayStatics.GetPlayerCharacter` 0))
  (bind _returnvalue_2 (`GameplayStatics.GetPlayerCharacter` 1))
  (bind _outactors (`GameplayStatics.GetAllActorsOfClassWithTag` "/Script/Engine.PlayerStart" "P1"))
  (bind _asbp_third_person_character_synty_final (cast `/Game/Blueprints/BP_ThirdPersonCharacterSynty_Final` _returnvalue))
  (set `/Game/Blueprints/BP_ThirdPersonCharacterSynty_Final.Index` 0 _asbp_third_person_character_synty_final)
  (`self.K2_SetActorTransform` _returnvalue (`self.GetTransform` (`|GetArrayItem` _outactors)) false true)
  (`GameplayStatics.CreatePlayer` 1)
  (`EnhancedInputSubsystemInterface.AddMappingContext` (pcsubsystem `EnhancedInputLocalPlayerSubsystem` (`GameplayStatics.GetPlayerController` 1)) "/Game/ThirdPerson/Input/IMC_Default_Player_2.IMC_Default_Player_2" 0 (struct))
  (bind _outactors_2 (`GameplayStatics.GetAllActorsOfClassWithTag` "/Script/Engine.PlayerStart" "P2"))
  (bind _asbp_third_person_character_synty_final_2 (cast `/Game/Blueprints/BP_ThirdPersonCharacterSynty_Final` _returnvalue_2))
  (set `/Game/Blueprints/BP_ThirdPersonCharacterSynty_Final.Index` 1 _asbp_third_person_character_synty_final_2)
  (`self.K2_SetActorTransform` _returnvalue_2 (`self.GetTransform` (`|GetArrayItem` _outactors_2)) false true))

(fn `UserConstructionScript`)