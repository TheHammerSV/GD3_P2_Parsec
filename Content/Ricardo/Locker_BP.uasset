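; Hideable locker the player enters and exits with the Hide input while inside its trigger box.
; Box overlap enables or disables input and gates Hide, which swings the door by timeline and runs ToggleHide.
; ToggleHide switches hiding state, character visibility and collision, and blends the view between character and locker.
; While hiding, look input drives clamped pitch and yaw, which a self-repeating MoveCamera event applies to the locker camera.
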(event `InputAction|Hide`
  (params (Key :type "Key Structure"))
  ;[1 1 1] Get In/Out of locker
  (:`Pressed`
    (`/Engine/EditorBlueprintResources/StandardMacros.Gate` true :!label _label
      (:`Exit`
        (`|ExecutionSequence`
          (:`then_0`
            (`self.ToggleHide`)
            (`KismetSystemLibrary.Delay` 0.2)
            (`self.EnableInput` (`GameplayStatics.GetPlayerController` 0) :!label _label_2)
            (goto _label :!via `Open`))
          (:`then_1`
            (bind (_direction _newtrack_0) (`Timeline|Open/Close Door` :!via `PlayFromStart`)
              (:`Update`
                (`SceneComponent.K2_SetRelativeRotation` (`self.Locker_Exterior`) (`KismetMathLibrary.MakeRotator` 0.0 0.0 (`KismetMathLibrary.Lerp` (`self.Close angle`) (`self.Open Angle`) _newtrack_0)) false false)))))))))

(event `self.Box.OnComponentBeginOverlap`
  (params (OverlappedComponent :type "PrimitiveComponent Object Reference") (OtherActor :type "Actor Object Reference") (OtherComp :type "PrimitiveComponent Object Reference") (OtherBodyIndex :type Integer) (bFromSweep :type Boolean) (SweepResult :type "HitResult Structure (by ref)"))
  ;[1 1 1] Get In/Out of locker
  (bind _asbp_third_person_character_synty_ric (cast `/Game/Ricardo/BP_ThirdPersonCharacterSynty_Ric` OtherActor))
  (set `self.CharacterRef` _asbp_third_person_character_synty_ric)
  (goto _label_2))

(event `self.Box.OnComponentEndOverlap`
  (params (OverlappedComponent :type "PrimitiveComponent Object Reference") (OtherActor :type "Actor Object Reference") (OtherComp :type "PrimitiveComponent Object Reference") (OtherBodyIndex :type Integer))
  ;[1 1 1] Get In/Out of locker
  (cast `/Game/Ricardo/BP_ThirdPersonCharacterSynty_Ric` OtherActor)
  (`self.DisableInput` (`GameplayStatics.GetPlayerController` 0))
  (goto _label :!via `Close`))

(event `InputAxis|Look Up`
  (params (AxisValue :type "Float (single-precision)"))
  ;[1 1 1] Move Camera
  (if (`self.IsHiding?`)
    (bind _output_get (set `self.Pitch` (`KismetMathLibrary.FClamp` (+ (`self.Pitch`) AxisValue) -40.0 20.0)))
    (else
      (`Pawn.AddControllerPitchInput` (`self.CharacterRef`) AxisValue))))

(event `MoveCamera`
  ;[1 1 1] Move Camera
  (if (`self.IsHiding?`)
    (`SceneComponent.K2_SetRelativeRotation` (`self.Camera`) (`KismetMathLibrary.MakeRotator` 0.0 (* (stale `InputAxis|Look Up` _output_get) -1.0) (stale `InputAxis|Turn` _output_get)) false false)
    (`KismetSystemLibrary.Delay` 0.001)
    (`self.MoveCamera`)))

(event `InputAxis|Turn`
  (params (AxisValue :type "Float (single-precision)"))
  ;[1 1 1] Move Camera
  (if (`self.IsHiding?`)
    (bind _output_get (set `self.Yaw` (`KismetMathLibrary.FClamp` (+ (`self.Yaw`) AxisValue) -60.0 60.0)))
    (else
      (`Pawn.AddControllerPitchInput` (`self.CharacterRef`) AxisValue))))

(fn `ToggleHide`
  (bind _returnvalue (`GameplayStatics.GetPlayerController` 0))
  (bind _characterref (`self.CharacterRef`))
  (if (`self.IsHiding?`)
    (set `self.IsHiding?` false)
    (`self.SetActorHiddenInGame` false)
    (`self.SetActorEnableCollision` _characterref true)
    (`PlayerController.SetViewTargetWithBlend` _returnvalue _characterref 0.6 "VTBlend_Linear" 0.0 false)
    (else
      (set `self.IsHiding?` true)
      (`self.SetActorHiddenInGame` _characterref true)
      (`self.SetActorEnableCollision` _characterref false)
      (`PlayerController.SetViewTargetWithBlend` _returnvalue self 0.6 "VTBlend_Linear" 0.0 false))))

(fn `UserConstructionScript`)