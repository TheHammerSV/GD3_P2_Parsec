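; GM_TwoPlayers is a game mode that sets up a local two-player session when play begins.
; On BeginPlay it teleports player 0's character to the first PlayerStart tagged P1, then creates a second local player.
; It then teleports that player's character to the first PlayerStart tagged P2, using actor tags to assign fixed spawn points.
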(event `self.ReceiveBeginPlay`
  (bind _outactors (`GameplayStatics.GetAllActorsOfClassWithTag` "/Script/Engine.PlayerStart" "P1"))
  (`self.K2_SetActorTransform` (`GameplayStatics.GetPlayerCharacter` 0) (`self.GetTransform` (`|GetArrayItem` _outactors)) false true)
  (`GameplayStatics.CreatePlayer` 1)
  (bind _outactors_2 (`GameplayStatics.GetAllActorsOfClassWithTag` "/Script/Engine.PlayerStart" "P2"))
  (`self.K2_SetActorTransform` (`GameplayStatics.GetPlayerCharacter` 1) (`self.GetTransform` (`|GetArrayItem` _outactors_2)) false true))

(fn `UserConstructionScript`)