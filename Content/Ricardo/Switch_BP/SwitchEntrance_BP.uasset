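; Switch entrance that lets a player carrying a KeyCard trigger the card release at the switch exit.
; Box overlap enables input and opens a gate only when the player character has KeyCard; otherwise, or on leaving, both are shut off.
; Pressing Spawn Item through the open gate calls SpitOutCard on the Switch_Exit_BP found in the level, then a timeline rotates the lid and shows the point light.
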(event `InputAction|Spawn Item`
  (params (Key :type "Key Structure"))
  (:`Pressed`
    (`KismetSystemLibrary.PrintString` "Hello")
    (`/Engine/EditorBlueprintResources/StandardMacros.Gate` true :!label _label
      (:`Exit`
        (bind _returnvalue (`GameplayStatics.GetActorOfClass` "/Game/Ricardo/Switch_BP/Switch_Exit_BP.Switch_Exit_BP_C"))
        (`/Game/Ricardo/Switch_BP/Switch_Exit_BP.SpitOutCard` _returnvalue)
        (bind (_direction _lid_shut) (`Timeline|LidShut`)
          (:`Update`
            (`SceneComponent.K2_SetRelativeRotation` (`self.BoxLid`) (`KismetMathLibrary.MakeRotator` _lid_shut) false false)
            (`SceneComponent.SetVisibility` (`self.PointLight`) true false)))))))

(event `self.Box.OnComponentBeginOverlap`
  (params (OverlappedComponent :type "PrimitiveComponent Object Reference") (OtherActor :type "Actor Object Reference") (OtherComp :type "PrimitiveComponent Object Reference") (OtherBodyIndex :type Integer) (bFromSweep :type Boolean) (SweepResult :type "HitResult Structure (by ref)"))
  (bind _returnvalue (`GameplayStatics.GetPlayerController` 0))
  (bind _asbp_third_person_character_synty_ric (cast `/Game/Ricardo/BP_ThirdPersonCharacterSynty_Ric` OtherActor))
  (if (`/Game/Ricardo/BP_ThirdPersonCharacterSynty_Ric.KeyCard` _asbp_third_person_character_synty_ric)
    (`self.EnableInput` _returnvalue)
    (`KismetSystemLibrary.PrintString` "Input Enabled")
    (goto _label :!via `Open`)
    (else
      (`self.DisableInput` _returnvalue :!label _label_2)
      (goto _label :!via `Close`))))

(event `self.Box.OnComponentEndOverlap`
  (params (OverlappedComponent :type "PrimitiveComponent Object Reference") (OtherActor :type "Actor Object Reference") (OtherComp :type "PrimitiveComponent Object Reference") (OtherBodyIndex :type Integer))
  (cast `/Game/Ricardo/BP_ThirdPersonCharacterSynty_Ric` OtherActor)
  (goto _label_2))

(fn `UserConstructionScript`)