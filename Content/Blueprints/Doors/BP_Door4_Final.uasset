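; BP_Door4_Final is an interactable door that swings open once when a player uses it.
; Tick sets the prompt text to "Press E to Open Door" until the door is open, then clears it.
; Use sets the Open flag, removes the player's interaction widget, plays an opening sound at world origin and runs a timeline that lerps the door's yaw to a quarter turn.
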(event `self.ReceiveTick`
  (params (DeltaSeconds :type "Float (single-precision)"))
  (if (`self.Open`)
    (set `self.WidgetText` "")
    (else
      (set `self.WidgetText` "Press E to Open Door"))))

(event `self.Use`
  (params (Player :type "/Game/Blueprints/BP_ThirdPersonCharacterSynty_Final Object Reference"))
  (if (not (`self.Open`))
    (set `self.Open` true)
    (`Widget.RemoveFromParent` (`/Game/Blueprints/BP_ThirdPersonCharacterSynty_Final.InteractableWidget` Player))
    (`GameplayStatics.PlaySoundAtLocation` "/Game/Ricardo/KeyCardAndDoor/Door_Sounds/spaceship-door-opening-43604.spaceship-door-opening-43604" (0.0 0.0 0.0) (struct) 1.0 1.0 0.0 null null null null)
    (bind (_direction _open_door) (`Timeline|OpenDoor`)
      (:`Update`
        (`SceneComponent.K2_SetRelativeRotation` (`self.Door`) (`KismetMathLibrary.MakeRotator` 0.0 0.0 (`KismetMathLibrary.Lerp` 0.0 90.0 _open_door)) false false)))))

(fn `UserConstructionScript`)